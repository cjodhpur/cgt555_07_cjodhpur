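; Base weapon Blueprint that handles firing, magazine ammo and reloading, with an empty WeaponTrace event as the hook for hit logic.
; FireWeapon spends a round, spawns particle and sound effects at the Arrow component, calls WeaponTrace, and auto-reloads on an empty magazine.
; Automatic and manual reloads share a DoOnce gate that blocks overlaps while a reload-bar widget animates and a delay refills ammo.
; It also exposes an FOV multiplier getter.
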(event `self.ReceiveBeginPlay`
  (set `self.Ammo` (`self.MaxMagazineAmmo`)))

(event `WeaponTrace`)

(event `/Game/Blueprints/FirstPersonTemplate/BPI_Weapon.FireWeapon`
  ;[1 1 1] FireWeaponLogic
  (if (<= (`self.Ammo`) 0)
    (`self.ReloadWeapon`)
    (else
      (set `self.Ammo` (- (`self.Ammo`) 1))
      (`self.WeaponFireEffects`)
      (`self.WeaponTrace`)
      (if (<= (`self.Ammo`) 0)
        (`self.ReloadWeapon`)))))

(event `ReloadWeapon`
  ;[1 1 1] Reload Weapon
  (`/Engine/EditorBlueprintResources/StandardMacros.DoOnce` false :!label _label
    (:`Completed`
      (bind _returnvalue (`|CreateWidget` "/Game/Blueprints/Weapons/WB_ReloadBar.WB_ReloadBar_C"))
      (`/Game/Blueprints/Weapons/WB_ReloadBar.ReloadAnimation` _returnvalue (`self.ReloadTime`))
      (`UserWidget.AddToViewport` _returnvalue 0)
      (`KismetSystemLibrary.Delay` (`self.ReloadTime`))
      (set `self.Ammo` (`self.MaxMagazineAmmo`))
      (goto _label :!via `Reset`))))

(event `/Game/Blueprints/FirstPersonTemplate/BPI_Weapon.Reload`
  ;[1 1 1] Reload Weapon
  (goto _label))

(fn `GetFOVMultiplier`
  (returns (FOVMultiplier :type "Float (double-precision)"))
  (return (`self.FOVMultiplier`)))

(fn `UserConstructionScript`)

(fn `WeaponFireEffects`
  (bind (_returnvalue_location _returnvalue_rotation) (`KismetMathLibrary.BreakTransform` (`SceneComponent.K2_GetComponentToWorld` (`self.Arrow`))))
  (`GameplayStatics.SpawnEmitterAtLocation` (`self.WeaponFireEmitter`) _returnvalue_location _returnvalue_rotation (`self.WeaponFireEmitterScale`))
  (`GameplayStatics.SpawnSoundAtLocation` (`self.WeaponFireSound`) _returnvalue_location (struct) 1.0 1.0 0.0 null null)
  (return))